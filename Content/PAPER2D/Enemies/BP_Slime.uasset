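; BP_Slime is a Paper2D slime enemy that turns its capsule and health bar toward the camera every tick.
; Pawn sensing sets a blackboard flag for three seconds on seeing the player, and Attack sphere-traces forward to deal damage with hit stop.
; Taking damage flashes the sprite through a timeline-driven dynamic material and launches it along the camera's view.
; Death spawns a small BP_Cube, then destroys the slime after a short delay.
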(event `self.ReceiveTick`
  (params (DeltaSeconds :type "Float (single-precision)"))
  (bind _health_bar_widget (`self.Health Bar Widget`))
  (bind _capsulecomponent (`self.CapsuleComponent`))
  (bind _aswb_slime_health_bar (cast `/Game/PAPER2D/Enemies/WB_SlimeHealthBar` (`WidgetComponent.GetWidget` (`self.Health Bar Widget`))))
  (`ProgressBar.SetPercent` (`/Game/PAPER2D/Enemies/WB_SlimeHealthBar.SlimeHealthBar` _aswb_slime_health_bar) (/ (`self.Health`) 3.0))
  (`SceneComponent.K2_SetWorldRotation` _health_bar_widget (`KismetMathLibrary.FindLookAtRotation` (`SceneComponent.K2_GetComponentLocation` _health_bar_widget) (`SceneComponent.K2_GetComponentLocation` (`PlayerCameraManager.TransformComponent` (`GameplayStatics.GetPlayerCameraManager` 0)))) false false)
  (`SceneComponent.K2_SetWorldRotation` _capsulecomponent (`KismetMathLibrary.FindLookAtRotation` (`SceneComponent.K2_GetComponentLocation` _capsulecomponent) (`SceneComponent.K2_GetComponentLocation` (`PlayerCameraManager.TransformComponent` (`GameplayStatics.GetPlayerCameraManager` 0)))) false false))

(event `self.ReceiveBeginPlay`
  (bind _returnvalue (`PrimitiveComponent.CreateDynamicMaterialInstance` (`self.Sprite`) 0 null "None"))
  (set `self.DynamicSpriteMat` _returnvalue))

(event `TriggerFlash`
  (params (FlashMultiplier :type "Float (single-precision)" :default 1.0) (FlashColour :type "LinearColor Structure" :default (struct :`R` 1.0 :`G` 0.926343 :`B` 0.981586 :`A` 1.0)) (PlayRate :type "Float (single-precision)" :default 5.0))
  (bind _dynamicspritemat (`self.DynamicSpriteMat`))
  (`MaterialInstanceDynamic.SetScalarParameterValue` _dynamicspritemat "FlashMultiplier" FlashMultiplier)
  (`MaterialInstanceDynamic.SetVectorParameterValue` _dynamicspritemat "FlashColour" FlashColour)
  (`TimelineComponent.SetPlayRate` (`self.FlashMultiplier`) PlayRate)
  (bind (_direction _alpha) (`Timeline|FlashMultiplier` :!via `PlayFromStart`)
    (:`Update`
      (`MaterialInstanceDynamic.SetScalarParameterValue` (`self.DynamicSpriteMat`) "FlashMultiplier" (`KismetMathLibrary.Lerp` 0.0 FlashMultiplier _alpha)))))

(event `self.PawnSensing.OnSeePawn`
  (params (Pawn :type "Pawn Object Reference"))
  (bind _returnvalue (`AIBlueprintHelperLibrary.GetBlackboard` (`AIBlueprintHelperLibrary.GetAIController` self)))
  (cast `/Game/PAPER2D/Character/TopDownCharBP` Pawn)
  (`BlackboardComponent.SetValueAsBool` _returnvalue "hasSeenPlayer" true)
  (`KismetSystemLibrary.Delay` 3.0)
  (`BlackboardComponent.SetValueAsBool` _returnvalue "hasSeenPlayer" false)
  (set `self.isAttacking` false)
  (set `self.isMoving` false))

(event `Attack`
  (bind _returnvalue (`self.K2_GetActorLocation`))
  (bind (_outhit _returnvalue_2) (`KismetSystemLibrary.SphereTraceSingleForObjects` _returnvalue (+ _returnvalue (* (`KismetMathLibrary.GetForwardVector` (`self.K2_GetActorRotation`)) 100.0)) 100.0 (`|MakeArray` "ObjectTypeQuery3" :!type "EObjectTypeQuery Enum")))
  (if _returnvalue_2
    (bind (_bblockinghit _binitialoverlap _time _distance _location _impactpoint _normal _impactnormal _physmat _hitactor) (`GameplayStatics.BreakHitResult` _outhit))
    (bind _astop_down_char_bp (cast `/Game/PAPER2D/Character/TopDownCharBP` _hitactor))
    (set `self.isAttacking` true)
    (`GameplayStatics.ApplyDamage` _hitactor 1.0)
    (`/Game/PAPER2D/Character/TopDownCharBP.StartHitStop` _astop_down_char_bp 0.1)
    (else
      (set `self.isAttacking` false))))

(event `self.ReceiveAnyDamage`
  (params (Damage :type "Float (single-precision)") (DamageType :type "DamageType Object Reference") (InstigatedBy :type "Controller Object Reference") (DamageCauser :type "Actor Object Reference"))
  (set `self.Health` (- (`self.Health`) Damage))
  (if (<= (`self.Health`) 0.0)
    (`GameplayStatics.PlaySound2D` "/Engine/EditorSounds/GamePreview/EndPlayInEditor_Cue.EndPlayInEditor_Cue" 1.0 1.0 0.0 null null)
    (`|SpawnActorFromClass` "/Game/PAPER2D/Cubes/_BP/BP_Cube.BP_Cube_C" (`KismetMathLibrary.MakeTransform` (`self.K2_GetActorLocation`) (struct) (0.2 0.2 0.2)) "AlwaysSpawn" "MultiplyWithRoot" null 0 null)
    (`KismetSystemLibrary.Delay` 0.5)
    (`self.K2_DestroyActor`)
    (else
      (`GameplayStatics.PlaySound2D` "/Engine/EditorSounds/GamePreview/StartSimulate_Cue.StartSimulate_Cue" 1.0 1.0 0.0 null null)
      (`self.TriggerFlash` 2.0 (struct :`R` 1.0 :`G` 0.926343 :`B` 0.981586 :`A` 1.0) 8.0)
      (`self.LaunchCharacter` (* (+ (`KismetMathLibrary.Conv_RotatorToVector` (`SceneComponent.K2_GetComponentRotation` (`PlayerCameraManager.TransformComponent` (`GameplayStatics.GetPlayerCameraManager` 0)))) (0.0 0.0 1.0)) (1500.0 1500.0 400.0))))))

(fn `UserConstructionScript`)